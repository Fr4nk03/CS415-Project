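; BP_Samurai is a 2D flipbook boss enemy that runs forward with Y pinned, turning at walls, and at edges unless chasing.
; AttackRange picks a short or long attack by SecondPhase, then damages the player after a delay if still inside DamageRange.
; Capsule contact hurts the player, or damages the boss if the player is attacking, triggering a looping launch and input lockout.
; DecreaseHealth handles hurt and death; ShootProjectile is defined but never called here.
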(event OnComponentBeginOverlap(WallDetector)
  (params (OverlappedComponent :type Primitive%20Component%20Object%20Reference) (OtherActor :type Actor%20Object%20Reference) (OtherComp :type Primitive%20Component%20Object%20Reference) (OtherBodyIndex :type Integer) (bFromSweep :type Boolean) (SweepResult :type Hit%20Result%20Structure%20%28by%20ref%29))
  ;[1 1 1] Wall Detector
  (CallFunction|TurnChar))

(event OnComponentEndOverlap(EdgeDetector)
  (params (OverlappedComponent :type Primitive%20Component%20Object%20Reference) (OtherActor :type Actor%20Object%20Reference) (OtherComp :type Primitive%20Component%20Object%20Reference) (OtherBodyIndex :type Integer))
  ;[1 1 1] Edge Detector
  (if (not (Variables|Default|GetIsChasing))
    (CallFunction|TurnChar)))

(event OnComponentBeginOverlap(DamageRange)
  (params (OverlappedComponent :type Primitive%20Component%20Object%20Reference) (OtherActor :type Actor%20Object%20Reference) (OtherComp :type Primitive%20Component%20Object%20Reference) (OtherBodyIndex :type Integer) (bFromSweep :type Boolean) (SweepResult :type Hit%20Result%20Structure%20%28by%20ref%29))
  (Utilities|Casting|CastToBP_Player OtherActor)
  (Variables|Default|SetPlayerInAttackRegion true))

(event OnComponentEndOverlap(DamageRange)
  (params (OverlappedComponent :type Primitive%20Component%20Object%20Reference) (OtherActor :type Actor%20Object%20Reference) (OtherComp :type Primitive%20Component%20Object%20Reference) (OtherBodyIndex :type Integer))
  (Variables|Default|SetPlayerInAttackRegion false))

(event OnComponentBeginOverlap(AttackRange)
  (params (OverlappedComponent :type Primitive%20Component%20Object%20Reference) (OtherActor :type Actor%20Object%20Reference) (OtherComp :type Primitive%20Component%20Object%20Reference) (OtherBodyIndex :type Integer) (bFromSweep :type Boolean) (SweepResult :type Hit%20Result%20Structure%20%28by%20ref%29))
  (bind _asbp_player (Utilities|Casting|CastToBP_Player OtherActor))
  (if (Variables|Default|GetSecondPhase)
    (CallFunction|LongAttack)
    (else
      (CallFunction|ShortAttack)))
  (Utilities|FlowControl|Delay 0.5)
  (if (Variables|Default|GetPlayerInAttackRegion)
    (Default|DecreaseHealth _asbp_player 3e+01))
  (Variables|Default|SetIsAttacking false)
  (Sprite|SetFlipbook (Variables|Default|GetSprite) "/Game/ArtAssets/Samurai__5_2D_Pixel_Art_v1_1/Sprites/Flipbook/Boss_Run.Boss_Run")
  (Variables|/Script/Engine.CharacterMovementComponent|SetMaxWalkSpeed (Variables|Character|GetCharacterMovement) 5e+02))

(event OnComponentBeginOverlap(CapsuleComponent)
  (params (OverlappedComponent :type Primitive%20Component%20Object%20Reference) (OtherActor :type Actor%20Object%20Reference) (OtherComp :type Primitive%20Component%20Object%20Reference) (OtherBodyIndex :type Integer) (bFromSweep :type Boolean) (SweepResult :type Hit%20Result%20Structure%20%28by%20ref%29))
  (bind _returnvalue (Transformation|GetActorLocation))
  (bind _returnvalue_2 (Transformation|GetActorLocation))
  (bind _returnvalue_3 (- _returnvalue _returnvalue_2))
  (bind _returnvalue_4 (Math|Vector|Normalize _returnvalue_3))
  (bind _returnvalue_5 (* _returnvalue_4 "500.000000,500.000000,0.000000"))
  (bind _asbp_player (Utilities|Casting|CastToBP_Player OtherActor))
  (if (Variables|/Game/Blueprints/BP_Player.BP_Player_C|GetIsAttacking _asbp_player)
    (CallFunction|DecreaseHealth 5e+01)
    (Character|LaunchCharacter _asbp_player (Math|Vector|MakeVector (.x _returnvalue_5) (.y _returnvalue_5) (+ (.z _returnvalue_5) 5e+01)) false false :!label _label)
    ;[1 1 1] Lose control for 0.2 scecond
    (Input|DisableInput _asbp_player 0)
    (Utilities|FlowControl|Delay 0.3)
    (Input|EnableInput _asbp_player 0)
    (goto _label)
    (else
      (Default|DecreaseHealth _asbp_player 1e+01))))

(event EventBeginPlay)

(event EventTick
  (params (DeltaSeconds :type Float%20%28single-precision%29))
  (bind _returnvalue (Transformation|GetActorLocation))
  (Pawn|Input|AddMovementInput (Transformation|GetActorForwardVector) 1.0 false)
  (Transformation|SetActorLocation (Math|Vector|MakeVector (.x _returnvalue) 0.0 (.z _returnvalue)) false false))

(fn ConstructionScript)

(fn TurnChar
  (Transformation|SetActorRotation (Math|Rotator|CombineRotators (Transformation|GetActorRotation) "0.000000,180.000000,0.000000")))

(fn DecreaseHealth
  (params (Damage :type Float%20%28double-precision%29))
  (bind _output_get (Variables|Default|SetHealth (- (Variables|Default|GetHealth) Damage)))
  (if (<= _output_get 0.0)
    (Sprite|SetFlipbook (Variables|Default|GetSprite) "/Game/ArtAssets/Samurai__5_2D_Pixel_Art_v1_1/Sprites/Flipbook/Boss_Death.Boss_Death")
    (Actor|SetLifeSpan 3.0)
    (Actor|DestroyActor)
    (else
      (Sprite|SetFlipbook (Variables|Default|GetSprite) "/Game/ArtAssets/Samurai__5_2D_Pixel_Art_v1_1/Sprites/Flipbook/Boss_Hurt.Boss_Hurt"))))

(fn ShootProjectile
  (Game|SpawnActorfromClass "/Game/Blueprints/Enemy1_Projectile.Enemy1_Projectile_C" (Math|Conversions|ToTransform(Vector) (Transformation|GetActorLocation)) "Undefined" "MultiplyWithRoot" 0 (* (Transformation|GetActorForwardVector) "1000.000000,0.000000,0.000000") 0)
  (Development|PrintString "Shoot"))

(fn ShortAttack
  (Variables|/Script/Engine.CharacterMovementComponent|SetMaxWalkSpeed (Variables|Character|GetCharacterMovement) 0.0)
  (Variables|Default|SetIsAttacking true)
  (Sprite|SetFlipbook (Variables|Default|GetSprite) "/Game/ArtAssets/Samurai__5_2D_Pixel_Art_v1_1/Sprites/Flipbook/Attack3.Attack3"))

(fn LongAttack
  (Sprite|SetFlipbook (Variables|Default|GetSprite) "/Game/ArtAssets/Samurai__5_2D_Pixel_Art_v1_1/Sprites/Flipbook/Attack1.Attack1"))