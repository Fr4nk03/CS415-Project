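; Paper2D transport actor that pushes the player along its forward vector, much like a conveyor belt.
; Begin and end overlap on its Box set and clear a Check flag without filtering which actor overlaps.
; Every Tick reapplies the FB_Trans flipbook and, while the flag is set, adds forward movement input to BP_Player, fetched as player character 0.
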(event OnComponentBeginOverlap(Box)
  (params (OverlappedComponent :type Primitive%20Component%20Object%20Reference) (OtherActor :type Actor%20Object%20Reference) (OtherComp :type Primitive%20Component%20Object%20Reference) (OtherBodyIndex :type Integer) (bFromSweep :type Boolean) (SweepResult :type Hit%20Result%20Structure%20%28by%20ref%29))
  (Variables|Default|Setcheck true))

(event OnComponentEndOverlap(Box)
  (params (OverlappedComponent :type Primitive%20Component%20Object%20Reference) (OtherActor :type Actor%20Object%20Reference) (OtherComp :type Primitive%20Component%20Object%20Reference) (OtherBodyIndex :type Integer))
  (Variables|Default|Setcheck false))

(event EventBeginPlay)

(event Collision|EventActorBeginOverlap
  (params (OtherActor :type Actor%20Object%20Reference)))

(event EventTick
  (params (DeltaSeconds :type Float%20%28single-precision%29))
  (Sprite|SetFlipbook (Variables|Default|GetRenderComponent) "/Game/Industrial_Zone_Tileset/4_Animated_objects/FB_Trans.FB_Trans")
  (if (Variables|Default|Getcheck)
    (bind _asbp_player (Utilities|Casting|CastToBP_Player (Game|GetPlayerCharacter 0)))
    (Pawn|Input|AddMovementInput _asbp_player (Transformation|GetActorForwardVector) 1.0 false)))

(fn ConstructionScript)