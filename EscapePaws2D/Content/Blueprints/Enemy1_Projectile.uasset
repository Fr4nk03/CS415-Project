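; Enemy projectile actor using a Paper2D flipbook, which damages the player on contact.
; Tick drives ProjectileMovement along VelocityVector in local space and resets the 3-second lifespan every frame, so that timer keeps restarting.
; Box overlap with BP_Player decreases health; overlap with either BP_Player or BP_industrial switches to the explosion flipbook.
; DestroyActor follows that switch immediately, overriding the short lifespan set for the explosion.
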(event OnComponentBeginOverlap(Box)
  (params (OverlappedComponent :type Primitive%20Component%20Object%20Reference) (OtherActor :type Actor%20Object%20Reference) (OtherComp :type Primitive%20Component%20Object%20Reference) (OtherBodyIndex :type Integer) (bFromSweep :type Boolean) (SweepResult :type Hit%20Result%20Structure%20%28by%20ref%29))
  (bind _asbp_player (Utilities|Casting|CastToBP_Player OtherActor)
    (:then
      (Default|DecreaseHealth _asbp_player 1e+01)
      (Sprite|SetFlipbook (Variables|Default|GetBlueProjectile) "/Game/ArtAssets/Explosions/Explosions/Blue/Sprites/BlueProjectileExplosion.BlueProjectileExplosion")
      (Actor|SetLifeSpan 1.0)
      (Actor|DestroyActor))
    (:CastFailed
      (Utilities|Casting|CastToBP_industrial OtherActor)
      (Sprite|SetFlipbook (Variables|Default|GetBlueProjectile) "/Game/ArtAssets/Explosions/Explosions/Blue/Sprites/BlueProjectileExplosion.BlueProjectileExplosion")
      (Actor|SetLifeSpan 1.0)
      (Actor|DestroyActor))))

(event EventBeginPlay)

(event Collision|EventActorBeginOverlap
  (params (OtherActor :type Actor%20Object%20Reference)))

(event EventTick
  (params (DeltaSeconds :type Float%20%28single-precision%29))
  (Game|Components|ProjectileMovement|SetVelocityinLocalSpace (Variables|Default|GetProjectileMovement) (Variables|Default|GetVelocityVector))
  (Actor|SetLifeSpan 3.0))

(fn ConstructionScript)