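; BP_enemy2 is a flipbook cyborg enemy that patrols back and forth and plays a punch animation when the player is in range.
; Tick moves it forward with the run flipbook, or stops movement input and shows the punch while Att is set.
; The Attack volume sets Att on player overlap, with no damage logic here.
; Turn rotates it 180 degrees when Wall touches a non-player or Box ends any overlap.
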(event OnComponentBeginOverlap(wall)
  (params (OverlappedComponent :type Primitive%20Component%20Object%20Reference) (OtherActor :type Actor%20Object%20Reference) (OtherComp :type Primitive%20Component%20Object%20Reference) (OtherBodyIndex :type Integer) (bFromSweep :type Boolean) (SweepResult :type Hit%20Result%20Structure%20%28by%20ref%29))
  (Utilities|Casting|CastToBP_Player OtherActor
    (:CastFailed
      (CallFunction|Turn))))

(event OnComponentEndOverlap(Box)
  (params (OverlappedComponent :type Primitive%20Component%20Object%20Reference) (OtherActor :type Actor%20Object%20Reference) (OtherComp :type Primitive%20Component%20Object%20Reference) (OtherBodyIndex :type Integer))
  (CallFunction|Turn))

(event OnComponentBeginOverlap(attack)
  (params (OverlappedComponent :type Primitive%20Component%20Object%20Reference) (OtherActor :type Actor%20Object%20Reference) (OtherComp :type Primitive%20Component%20Object%20Reference) (OtherBodyIndex :type Integer) (bFromSweep :type Boolean) (SweepResult :type Hit%20Result%20Structure%20%28by%20ref%29))
  (Utilities|Casting|CastToBP_Player OtherActor)
  (Variables|Default|Setatt true))

(event OnComponentEndOverlap(attack)
  (params (OverlappedComponent :type Primitive%20Component%20Object%20Reference) (OtherActor :type Actor%20Object%20Reference) (OtherComp :type Primitive%20Component%20Object%20Reference) (OtherBodyIndex :type Integer))
  (Utilities|Casting|CastToBP_Player OtherActor)
  (Variables|Default|Setatt false))

(event EventBeginPlay)

(event Collision|EventActorBeginOverlap
  (params (OtherActor :type Actor%20Object%20Reference)))

(event EventTick
  (params (DeltaSeconds :type Float%20%28single-precision%29))
  (if (Variables|Default|Getatt)
    (Sprite|SetFlipbook (Variables|Default|GetSprite) "/Game/ArtAssets/enemy/Flipbooks/FB_CyborgPunch.FB_CyborgPunch")
    (else
      (Sprite|SetFlipbook (Variables|Default|GetSprite) "/Game/ArtAssets/enemy/Flipbooks/FB_CyborgRun.FB_CyborgRun")
      (Pawn|Input|AddMovementInput (Transformation|GetActorForwardVector) 1.0 false))))

(fn ConstructionScript)

(fn Turn
  (Transformation|SetActorRotation (Math|Rotator|CombineRotators (Transformation|GetActorRotation) "0.000000,180.000000,0.000000")))