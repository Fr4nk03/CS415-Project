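; BP_Enemy1 is a flipbook-sprite patrol enemy that damages the player on contact and shoots projectiles.
; Wall and edge detector overlaps flip its facing, with edge turns suppressed while chasing; MoveForward supplies movement input.
; PlayerDetector knocks the player back and briefly disables input.
; Entering PursureDetector turns it toward the player, fires one projectile and starts chasing; its DecreaseHealth has no death handling yet.
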(event OnComponentBeginOverlap(WallDetector)
  (params (OverlappedComponent :type Primitive%20Component%20Object%20Reference) (OtherActor :type Actor%20Object%20Reference) (OtherComp :type Primitive%20Component%20Object%20Reference) (OtherBodyIndex :type Integer) (bFromSweep :type Boolean) (SweepResult :type Hit%20Result%20Structure%20%28by%20ref%29))
  ;[1 1 1] Wall Detector
  (CallFunction|TurnChar))

(event OnComponentEndOverlap(EdgeDetector)
  (params (OverlappedComponent :type Primitive%20Component%20Object%20Reference) (OtherActor :type Actor%20Object%20Reference) (OtherComp :type Primitive%20Component%20Object%20Reference) (OtherBodyIndex :type Integer))
  ;[1 1 1] Edge Detector
  (if (not (Variables|Default|GetIsChasing))
    (CallFunction|TurnChar)))

(event OnComponentBeginOverlap(PlayerDetector)
  (params (OverlappedComponent :type Primitive%20Component%20Object%20Reference) (OtherActor :type Actor%20Object%20Reference) (OtherComp :type Primitive%20Component%20Object%20Reference) (OtherBodyIndex :type Integer) (bFromSweep :type Boolean) (SweepResult :type Hit%20Result%20Structure%20%28by%20ref%29))
  (bind _returnvalue (Transformation|GetActorLocation OtherActor))
  (bind _returnvalue_2 (Transformation|GetActorLocation))
  (bind _returnvalue_3 (- _returnvalue _returnvalue_2))
  (bind _returnvalue_4 (Math|Vector|Normalize _returnvalue_3))
  (bind _returnvalue_5 (* _returnvalue_4 "500.000000,500.000000,0.000000"))
  ;[1 1 1] Knock Back Player
  (bind _asbp_player (Utilities|Casting|CastToBP_Player OtherActor))
  (Default|DecreaseHealth _asbp_player 1e+01)
  (Development|PrintString "Hit player!")
  (Character|LaunchCharacter _asbp_player (Math|Vector|MakeVector (.x _returnvalue_5) (.y _returnvalue_5) (+ (.z _returnvalue_5) 5e+01)) false false)
  (Effects|SpawnEmitteratLocation 0 (Transformation|GetActorLocation))
  ;[1 1 1] Lose control for 0.2 scecond
  (Input|DisableInput _asbp_player 0)
  (Utilities|FlowControl|Delay 0.3)
  (Input|EnableInput _asbp_player 0))

(event OnComponentBeginOverlap(PursureDetector)
  (params (OverlappedComponent :type Primitive%20Component%20Object%20Reference) (OtherActor :type Actor%20Object%20Reference) (OtherComp :type Primitive%20Component%20Object%20Reference) (OtherBodyIndex :type Integer) (bFromSweep :type Boolean) (SweepResult :type Hit%20Result%20Structure%20%28by%20ref%29))
  (bind _returnvalue (Transformation|GetActorForwardVector))
  (bind _returnvalue_2 (> (.x _returnvalue) 0.0))
  ;[1 1 1] Chase Player and Shoot Projectiles
  (bind _asbp_player (Utilities|Casting|CastToBP_Player OtherActor))
  (Sprite|SetFlipbook (Variables|Default|GetSprite) "/Game/ArtAssets/EnemyAssets/Flipbooks/FB_Enemy1_Shoot.FB_Enemy1_Shoot")
  (CallFunction|ShootProjectile)
  (Variables|Default|SetIsChasing true)
  (if (< (.x (Transformation|GetActorLocation _asbp_player)) (.x (Transformation|GetActorLocation)))
    (if _returnvalue_2
      (CallFunction|TurnChar))
    (elif (not _returnvalue_2)
      (CallFunction|TurnChar))))

(event OnComponentEndOverlap(PursureDetector)
  (params (OverlappedComponent :type Primitive%20Component%20Object%20Reference) (OtherActor :type Actor%20Object%20Reference) (OtherComp :type Primitive%20Component%20Object%20Reference) (OtherBodyIndex :type Integer))
  ;[1 1 1] Stop Chasing
  (Utilities|Casting|CastToBP_Player OtherActor)
  (Variables|Default|SetIsChasing false)
  (Sprite|SetFlipbook (Variables|Default|GetSprite) "/Game/ArtAssets/EnemyAssets/Flipbooks/FB_Enemy1_Run.FB_Enemy1_Run"))

(event Custom|MoveForward
  (Pawn|Input|AddMovementInput (Transformation|GetActorForwardVector) 1.0 false))

(event EventBeginPlay)

(event EventTick
  (params (DeltaSeconds :type Float%20%28single-precision%29)))

(fn ConstructionScript)

(fn TurnChar
  (Transformation|SetActorRotation (Math|Rotator|CombineRotators (Transformation|GetActorRotation) "0.000000,180.000000,0.000000")))

(fn DecreaseHealth
  (params (Damage :type Float%20%28double-precision%29))
  (bind _output_get (Variables|Default|SetHealth (- (Variables|Default|GetHealth) Damage)))
  (if (<= _output_get 0.0)
    _))

(fn ShootProjectile
  (Game|SpawnActorfromClass "/Game/Blueprints/Enemy1_Projectile.Enemy1_Projectile_C" (Math|Conversions|ToTransform(Vector) (Transformation|GetActorLocation)) "Undefined" "MultiplyWithRoot" 0 (* (Transformation|GetActorForwardVector) "1000.000000,0.000000,0.000000") 0)
  (Development|PrintString "Shoot"))