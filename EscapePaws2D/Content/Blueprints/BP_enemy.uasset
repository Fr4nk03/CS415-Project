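; BP_enemy is a flipbook bike enemy that patrols forward and damages the player on contact.
; It reverses via Turn when Wall overlaps a non-player or Box stops overlapping.
; The Attack overlap damages BP_Player once on entry and toggles its damage flag plus Att, which makes Tick halt movement and swap run for attack animation.
; DecreaseHealth tracks its health, destroying it with a death sound at zero.
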(event OnComponentBeginOverlap(wall)
  (params (OverlappedComponent :type Primitive%20Component%20Object%20Reference) (OtherActor :type Actor%20Object%20Reference) (OtherComp :type Primitive%20Component%20Object%20Reference) (OtherBodyIndex :type Integer) (bFromSweep :type Boolean) (SweepResult :type Hit%20Result%20Structure%20%28by%20ref%29))
  (Utilities|Casting|CastToBP_Player OtherActor
    (:CastFailed
      (CallFunction|Turn))))

(event OnComponentEndOverlap(Box)
  (params (OverlappedComponent :type Primitive%20Component%20Object%20Reference) (OtherActor :type Actor%20Object%20Reference) (OtherComp :type Primitive%20Component%20Object%20Reference) (OtherBodyIndex :type Integer))
  (CallFunction|Turn))

(event OnComponentBeginOverlap(attack)
  (params (OverlappedComponent :type Primitive%20Component%20Object%20Reference) (OtherActor :type Actor%20Object%20Reference) (OtherComp :type Primitive%20Component%20Object%20Reference) (OtherBodyIndex :type Integer) (bFromSweep :type Boolean) (SweepResult :type Hit%20Result%20Structure%20%28by%20ref%29))
  (bind _asbp_player (Utilities|Casting|CastToBP_Player OtherActor))
  (Default|DecreaseHealth _asbp_player 2e+01)
  (Variables|/Game/Blueprints/BP_Player.BP_Player_C|SetIsTakingDamage _asbp_player true)
  (Variables|Default|Setatt true))

(event OnComponentEndOverlap(attack)
  (params (OverlappedComponent :type Primitive%20Component%20Object%20Reference) (OtherActor :type Actor%20Object%20Reference) (OtherComp :type Primitive%20Component%20Object%20Reference) (OtherBodyIndex :type Integer))
  (bind _asbp_player (Utilities|Casting|CastToBP_Player OtherActor))
  (Variables|/Game/Blueprints/BP_Player.BP_Player_C|SetIsTakingDamage _asbp_player false)
  (Variables|Default|Setatt false))

(event EventBeginPlay)

(event Collision|EventActorBeginOverlap
  (params (OtherActor :type Actor%20Object%20Reference)))

(event EventTick
  (params (DeltaSeconds :type Float%20%28single-precision%29))
  (if (Variables|Default|Getatt)
    (Sprite|SetFlipbook (Variables|Default|GetSprite) "/Game/ArtAssets/enemy/Sprite/Bike_attack.Bike_attack")
    (else
      (Sprite|SetFlipbook (Variables|Default|GetSprite) "/Game/ArtAssets/enemy/Sprite/Bike_run.Bike_run")
      (Pawn|Input|AddMovementInput (Transformation|GetActorForwardVector) 1.0 false))))

(fn ConstructionScript)

(fn Turn
  (Transformation|SetActorRotation (Math|Rotator|CombineRotators (Transformation|GetActorRotation) "0.000000,180.000000,0.000000")))

(fn DecreaseHealth
  (params (damage :type Float%20%28double-precision%29))
  (if (<= (- (Variables|Default|Gethealth) damage) 0.0)
    (Actor|DestroyActor)
    (Audio|PlaySound2D "/Game/ArtAssets/Sound/mixkit-enemy-death-voice-3168.mixkit-enemy-death-voice-3168" 1.0 1.0 0.0 0 0)
    (else
      (Variables|Default|Sethealth (- (Variables|Default|Gethealth) damage)))))